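; Base dungeon character Blueprint with a sprite that handles taking damage and hit feedback.
; While not defeated, incoming damage lowers health through BPCHealth, knocks the character away from the attacker via a timeline-driven velocity, and briefly flashes the sprite red.
; A character attacker gets hit stop by zeroing its custom time dilation, then an empty HandleHitExtended hook runs.
; A hit-animation stun and defeat-jump chain exists but is unconnected.
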(event Custom|GetKnockedBack
  (params (Attacker :type Actor%20Object%20Reference))
  (Variables|Default|SetKnockBackDirection (Math|Vector|GetForwardVector (Math|Rotator|FindLookatRotation (Transformation|GetActorLocation Attacker) (Transformation|GetActorLocation))))
  (Components|Timeline|SetPlayRate (Variables|Default|GetKnockBackmovement) 5.0)
  (Timeline|KnockBackMovement PlayFromStart
    (:Update
      (Variables|/Script/Engine.MovementComponent|SetVelocity (Variables|Character|GetCharacterMovement) (* (Variables|Default|GetKnockBackDirection) (Variables|Default|GetKnockBackStrength) (Utilities|Time|GetWorldDeltaSeconds))))))

(event Custom|FlashSprite
  (Sprite|SetSpriteColor (Variables|Default|GetSprite) "(R=1.000000,G=0.000000,B=0.000000,A=1.000000)")
  (Utilities|FlowControl|RetriggerableDelay 0.2)
  (Sprite|SetSpriteColor (Variables|Default|GetSprite) "(R=1.000000,G=1.000000,B=1.000000,A=1.000000)"))

(event Custom|HitStop
  (Variables|Default|SetCustomTimeDilation 0.0)
  (Utilities|FlowControl|RetriggerableDelay (Variables|Default|GetHitStopDuration))
  (Variables|Default|SetCustomTimeDilation 1.0))

(event EventBeginPlay)

(event Collision|EventActorBeginOverlap
  (params (OtherActor :type Actor%20Object%20Reference)))

(event EventTick
  (params (DeltaSeconds :type Float%20%28single-precision%29)))

(event Game|Damage|EventAnyDamage
  (params (Damage :type Float%20%28single-precision%29) (DamageType :type Damage%20Type%20Object%20Reference) (InstigatedBy :type Controller%20Object%20Reference) (DamageCauser :type Actor%20Object%20Reference))
  (if (not (Variables|/Game/Blueprints/Components/BPC_Health.BPC_Health_C|GetIsDefeated (Variables|Default|GetBPC_Health)))
    (Default|DecreaseHealth (Variables|Default|GetBPC_Health) Damage)
    (CallFunction|GetKnockedBack DamageCauser)
    (CallFunction|FlashSprite)
    (bind _asbp_dungeon_char_base (Utilities|Casting|CastToBP_DungeonChar_BASE DamageCauser))
    (CallFunction|HitStop _asbp_dungeon_char_base)
    (CallFunction|HandleHitExtended)))

(fn ConstructionScript)

(fn HandleHitExtended)