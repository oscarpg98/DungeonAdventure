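; BPC_Health is a health component that tracks an owner's current health, defeat state and temporary invincibility.
; Health fills to maximum on BeginPlay, and DecreaseHealth subtracts damage clamped at zero and flags defeat when it runs out.
; SetInvincibility uses a retriggerable delay, so repeat calls restart the window before it calls InvincibilityExpired.
; CanBeDamaged reports true only while neither defeated nor invincible, though DecreaseHealth does not check it itself.
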(event Custom|SetInvincibility
  (Variables|Default|SetIsInvincible true)
  (Utilities|FlowControl|RetriggerableDelay (Variables|Default|GetinvincibilityDuration))
  (Variables|Default|SetIsInvincible false)
  (Default|CallInvincibilityExpired))

(event EventBeginPlay
  (Variables|Default|SetCurrentHealth (Variables|Default|GetMaxHealth)))

(event EventTick
  (params (DeltaSeconds :type Float%20%28single-precision%29)))

(fn DecreaseHealth
  (params (IncomingDamage :type Float%20%28double-precision%29))
  (Variables|Default|SetCurrentHealth (Math|Float|Max(Float) (- (Variables|Default|GetCurrentHealth) IncomingDamage) 0.0))
  (Variables|Default|SetIsDefeated (<= (Variables|Default|GetCurrentHealth) 0.0)))

(fn CanbeDamaged
  (return (and (not (Variables|Default|GetIsDefeated)) (not (Variables|Default|GetIsInvincible)))))